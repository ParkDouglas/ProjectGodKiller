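; Moving melee enemy that chases the player once PawnSensing spots a pawn and damages them on reaching them.
; Each sighting sets a seeing flag, never cleared here, and calls FollowPlayer, which runs AIMoveTo toward the player character.
; Successful moves apply damage to the BP_Player reference cached only by the Hit event.
; A CanAttack flag with a delay gates attacks, though every FollowPlayer call re-enables it.
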(event `self.PawnSensing.OnSeePawn`
  (params (Pawn :type "Pawn Object Reference"))
  ;[1 1 1] Follow player and attak if in range
  (set `self.IsSeeingPlayer` true)
  (`self.FollowPlayer`))

(event `FollowPlayer`
  ;[1 1 1] Follow player and attak if in range
  (set `self.CanAttack` true)
  (if (`self.IsSeeingPlayer`)
    (`|AIMoveTo` self (0.0 0.0 0.0) (`GameplayStatics.GetPlayerCharacter` 0)
      (:`OnSuccess`
        (if (`self.CanAttack`)
          (set `self.CanAttack` false)
          (`GameplayStatics.ApplyDamage` (stale `self.ReceiveHit` _asbp_player) 10.0)
          (`KismetSystemLibrary.Delay` 1.0)
          (set `self.CanAttack` true))))))

(event `self.ReceiveHit`
  (params (MyComp :type "PrimitiveComponent Object Reference") (Other :type "Actor Object Reference") (OtherComp :type "PrimitiveComponent Object Reference") (bSelfMoved :type Boolean) (HitLocation :type "Vector Structure") (HitNormal :type "Vector Structure") (NormalImpulse :type "Vector Structure") (Hit :type "HitResult Structure (by ref)"))
  ;[1 1 1] Follow player and attak if in range
  (bind _asbp_player (cast `/Game/BluePrints/BP_Player` Other)))

(fn `UserConstructionScript`)