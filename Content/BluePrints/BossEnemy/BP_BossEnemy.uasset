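; BP_BossEnemy is a boss that shoots at the player and opens the YouWin level when its health runs out.
; PawnSensing turns it toward a seen player and, if CanAttack, spawns a bullet.
; Shooting and player hits share one damage-and-cooldown chain targeting the Hit event's player cast, but hits skip the CanAttack check.
; AnyDamage reduces BossHealth and destroys the boss at zero.
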(event `self.PawnSensing.OnSeePawn`
  (params (Pawn :type "Pawn Object Reference"))
  ;[1 1 1] Enemy rotate to shoot at player
  (bind _asbp_player (cast `/Game/BluePrints/BP_Player` Pawn))
  (`self.K2_SetActorRotation` (`KismetMathLibrary.FindLookAtRotation` (`self.K2_GetActorLocation`) (`self.K2_GetActorLocation` _asbp_player)))
  (if (`self.CanAttack`)
    (`|SpawnActorFromClass` "/Game/BluePrints/BossEnemy/BP_EnemyBullet.BP_EnemyBullet_C" (`SceneComponent.K2_GetComponentToWorld` (`self.SpawnPoint`)) "Undefined" "MultiplyWithRoot" null null)
    (`GameplayStatics.ApplyDamage` (stale `self.ReceiveHit` _asbp_player) 5.0 :!label _label)
    (set `self.CanAttack` false)
    (`KismetSystemLibrary.Delay` 1.0)
    (set `self.CanAttack` true)))

(event `self.ReceiveHit`
  (params (MyComp :type "PrimitiveComponent Object Reference") (Other :type "Actor Object Reference") (OtherComp :type "PrimitiveComponent Object Reference") (bSelfMoved :type Boolean) (HitLocation :type "Vector Structure") (HitNormal :type "Vector Structure") (NormalImpulse :type "Vector Structure") (Hit :type "HitResult Structure (by ref)"))
  ;[1 1 1] Enemy rotate to shoot at player
  (bind _asbp_player (cast `/Game/BluePrints/BP_Player` Other))
  (goto _label))

(event `self.ReceiveAnyDamage`
  (params (Damage :type "Float (single-precision)") (DamageType :type "DamageType Object Reference") (InstigatedBy :type "Controller Object Reference") (DamageCauser :type "Actor Object Reference"))
  ;[1 1 1] Take damage enemy
  (bind _output_get (set `self.BossHealth` (- (`self.BossHealth`) Damage)))
  (if (<= _output_get 0.0)
    (`self.K2_DestroyActor`)
    (`GameplayStatics.OpenLevel` "YouWin")))

(fn `UserConstructionScript`)