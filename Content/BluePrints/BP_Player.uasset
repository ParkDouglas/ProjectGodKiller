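; BP_Player is the player Character, with axis-driven movement, mouse or stick style look, and a dash.
; Movement follows the actor's forward and right vectors, while look feeds controller yaw and pitch.
; Dash launches the character along a scaled copy of its horizontal velocity, so it does nothing from standstill.
; Two dashes are allowed before a short delay resets the counter, and spawning prints a debug message.
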(event `self.ReceiveBeginPlay`
  ;[1 1 1] Print to screen player spawned
  (`KismetSystemLibrary.PrintString` "BP_PlayerSpawned" true true (struct :`R` 1.0 :`B` 0.996378 :`A` 1.0) 5.0))

(event `InputAxis|MoveForward`
  (params (AxisValue :type "Float (single-precision)"))
  ;[1 1 1] Movement
  (`self.AddMovementInput` (`self.GetActorForwardVector`) AxisValue))

(event `InputAxis|MoveHorizontal`
  (params (AxisValue :type "Float (single-precision)"))
  ;[1 1 1] Movement
  (`self.AddMovementInput` (`self.GetActorRightVector`) AxisValue))

(event `InputAxis|LookHorizontal`
  (params (AxisValue :type "Float (single-precision)"))
  ;[1 1 1] Look
  (`self.AddControllerYawInput` AxisValue))

(event `InputAxis|LookVertical`
  (params (AxisValue :type "Float (single-precision)"))
  ;[1 1 1] Look
  (`self.AddControllerPitchInput` AxisValue))

(event `InputAction|Dash`
  (params (Key :type "Key Structure"))
  (bind (_returnvalue_x _returnvalue_y) (`KismetMathLibrary.BreakVector` (`self.GetVelocity`)))
  ;[1 1 1] dash
  (:`Pressed`
    (if (!= (`self.DashUsed`) 2)
      (`self.LaunchCharacter` (* (`KismetMathLibrary.MakeVector` _returnvalue_x _returnvalue_y) 10))
      (bind _result (`/Engine/EditorBlueprintResources/StandardMacros.IncrementInt` (`self.DashUsed`))
        (:`  `
          (if (== _result 2)
            (`KismetSystemLibrary.Delay` 2.0)
            (set `self.DashUsed` 0)))))))

(fn `UserConstructionScript`)